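; SS_ExitDoor_BP is an exit door that opens when a character enters its collision volume and closes when they leave.
; Overlaps filter by "character" in the actor's display name, then play a sound and run or reverse the OpenDoor timeline, lerping the door's relative location.
; Those relative locations also position the sounds.
; The opening branch is always true; a player Score check exists but is unused.
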(event OnComponentBeginOverlap(Collision)
  (params (OverlappedComponent :type Primitive%20Component%20Object%20Reference) (OtherActor :type Actor%20Object%20Reference) (OtherComp :type Primitive%20Component%20Object%20Reference) (OtherBodyIndex :type Integer) (bFromSweep :type Boolean) (SweepResult :type Hit%20Result%20Structure%20%28by%20ref%29))
  ;[1 1 1] Opens Door
  (if true
    (if (Utilities|String|Contains (Utilities|GetDisplayName OtherActor) "character")
      (Audio|PlaySoundatLocation "/Game/Audio/Sliding_Door/garage_door_open_new.garage_door_open_new" (Variables|Default|GetDoorLocationBegin) "0, 0, 0" 1.0 1.0 0.0 0 0 0)
      (bind _raisedoor (Timeline|OpenDoor Play)
        (:Update
          (Transformation|SetRelativeLocation (Variables|Default|GetDoor) (Math|Vector|Lerp(Vector) (Variables|Default|GetDoorLocationBegin) (Variables|Default|GetDoorLocationEnd) _raisedoor) false false))))))

(event OnComponentEndOverlap(Collision)
  (params (OverlappedComponent :type Primitive%20Component%20Object%20Reference) (OtherActor :type Actor%20Object%20Reference) (OtherComp :type Primitive%20Component%20Object%20Reference) (OtherBodyIndex :type Integer))
  ;[1 1 1] Opens Door
  (if (Utilities|String|Contains (Utilities|GetDisplayName OtherActor) "character")
    (Audio|PlaySoundatLocation "/Game/Audio/Sliding_Door/garage-door-closed-edited.garage-door-closed-edited" (Variables|Default|GetDoorLocationEnd) "0, 0, 0" 1.0 1.0 0.0 0 0 0)
    (bind _raisedoor (Timeline|OpenDoor Reverse)
      (:Update
        (Transformation|SetRelativeLocation (Variables|Default|GetDoor) (Math|Vector|Lerp(Vector) (Variables|Default|GetDoorLocationBegin) (Variables|Default|GetDoorLocationEnd) _raisedoor) false false)))))

(event EventBeginPlay
  ;[1 1 1] Gets and Sets Door Location
  (Variables|Default|SetDoorLocationBegin (Variables|/Script/Engine.SceneComponent|GetRelativeLocation (Variables|Default|GetDoor))))

(event Collision|EventActorBeginOverlap
  (params (OtherActor :type Actor%20Object%20Reference)))

(event EventTick
  (params (DeltaSeconds :type Float%20%28single-precision%29)))

(fn ConstructionScript)