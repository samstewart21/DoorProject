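; SSPlatform_BP is a platform that rises when a character enters its collision volume and lowers when it leaves.
; BeginPlay stores the platform's relative location as the start point.
; Overlaps play or reverse the Platform_Up timeline, whose Rise track lerps the platform between that start and PlatformEnd, without sweeping.
; Characters are detected by searching the overlapping actor's object name for "character" rather than by casting.
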(event OnComponentBeginOverlap(Collision_Platform)
  (params (OverlappedComponent :type Primitive%20Component%20Object%20Reference) (OtherActor :type Actor%20Object%20Reference) (OtherComp :type Primitive%20Component%20Object%20Reference) (OtherBodyIndex :type Integer) (bFromSweep :type Boolean) (SweepResult :type Hit%20Result%20Structure%20%28by%20ref%29))
  ;[1 1 1] Raises and Lowers Platform
  (if (Utilities|String|Contains (Utilities|GetObjectName OtherActor) "character")
    (bind _rise (Timeline|Platform_Up Play)
      (:Update
        (Transformation|SetRelativeLocation (Variables|Default|GetPlatform) (Math|Vector|Lerp(Vector) (Variables|Default|GetPlatformBegin) (Variables|Default|GetPlatformEnd) _rise) false false)))))

(event OnComponentEndOverlap(Collision_Platform)
  (params (OverlappedComponent :type Primitive%20Component%20Object%20Reference) (OtherActor :type Actor%20Object%20Reference) (OtherComp :type Primitive%20Component%20Object%20Reference) (OtherBodyIndex :type Integer))
  ;[1 1 1] Raises and Lowers Platform
  (if (Utilities|String|Contains (Utilities|GetObjectName OtherActor) "character")
    (bind _rise (Timeline|Platform_Up Reverse)
      (:Update
        (Transformation|SetRelativeLocation (Variables|Default|GetPlatform) (Math|Vector|Lerp(Vector) (Variables|Default|GetPlatformBegin) (Variables|Default|GetPlatformEnd) _rise) false false)))))

(event EventBeginPlay
  ;[1 1 1] Gets and Sets Platform Location
  (Variables|Default|SetPlatformBegin (Variables|/Script/Engine.SceneComponent|GetRelativeLocation (Variables|Default|GetPlatform))))

(event Collision|EventActorBeginOverlap
  (params (OtherActor :type Actor%20Object%20Reference)))

(event EventTick
  (params (DeltaSeconds :type Float%20%28single-precision%29)))

(fn ConstructionScript)