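; Level player controller that toggles the pause menu on the Pause input action.
; With no valid menu reference, it creates the Stewart_PauseMenu widget, shows the cursor, allows game and UI input, pauses the game and hides the FirstPersonCharacter's HUD.
; Otherwise it removes and clears the menu, restores game-only input, hides the cursor, unpauses and turns the HUD back on.
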(event Input|ActionEvents|InputActionPause
  (params (Key :type Key%20Structure :default "None"))
  (bind _returnvalue (Game|GetPlayerController 0))
  (bind _returnvalue_2 (Game|GetPlayerController 0))
  ;[1 1 1] When the P key is pressed checks to see if HUD is there, if it is destroys it and recreates it, if not it creates it.  Also pauses the game when the pause menu is displayed and removes HUD  and unpauses game and readds HUD when game is unpaused.
  (:Pressed
    (Utilities|IsValid (Variables|Default|GetPauseUIRef2)
      (:Is%20Valid
        (Widget|RemovefromParent (Variables|Default|GetPauseUIRef2))
        (Variables|Default|SetPauseUIRef2 0)
        (Input|SetInputModeGameOnly _returnvalue_2)
        (Variables|/Script/Engine.PlayerController|SetbShowMouseCursor _returnvalue_2 false)
        (Game|SetGamePaused false)
        (Default|ToggleHUDon (.AsFirst%20Person%20Character (Utilities|Casting|CastToFirstPersonCharacter (Game|GetPlayerCharacter 0)))))
      (:Is%20Not%20Valid
        (bind _returnvalue_3 (UserInterface|CreateWidget "/Game/Widgets/Stewart_PauseMenu.Stewart_PauseMenu_C"))
        (bind _output_get (Variables|Default|SetPauseUIRef2 _returnvalue_3))
        (UserInterface|Viewport|AddtoViewport _output_get 0)
        (Input|SetInputModeGameandUI _returnvalue 0 "DoNotLock" true)
        (Variables|/Script/Engine.PlayerController|SetbShowMouseCursor _returnvalue true)
        (Game|SetGamePaused true)
        (Default|ToggleHUDOff (.AsFirst%20Person%20Character (Utilities|Casting|CastToFirstPersonCharacter (Game|GetPlayerCharacter 0))))))))

(fn ConstructionScript)